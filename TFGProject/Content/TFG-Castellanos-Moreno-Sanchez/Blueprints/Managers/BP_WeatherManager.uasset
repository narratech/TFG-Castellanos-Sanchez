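; BP_WeatherManager is a weather manager that turns rain on and off within a set time-of-day window.
; On BeginPlay it gives the volumetric clouds a dynamic material and starts a looping timer that checks the LightingManager's time of day.
; Entering or leaving the window plays or reverses a timeline that drives the StormClouds material parameter.
; The Niagara rain system activates or deactivates only when that cloud transition finishes.
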(event Custom|ComprobarClima
  (bind _sistemalluvia (Variables|Referencias|GetSistemaLluvia))
  (bind _niagaracomponent (Variables|/Script/Niagara.NiagaraActor|GetNiagaraComponent _sistemalluvia))
  (if (Math|Float|InRange(Float) (Variables|/Game/PWL_Light_Manager/Blueprint/BP_Lighting_Manager.BP_Lighting_Manager_C|GetSun%20Height%20%28Time%20Of%20Day%29 (Variables|Referencias|GetLightingManager)) (Variables|Default|GetHoraDeLluvia) (Variables|Default|GetHoraFinLluvia))
    (if (not (Variables|Default|GetEstaLloviendo))
      (Variables|Default|SetEstaLloviendo true)
      (bind _intensidadtormenta (Timeline|TransiciónClima Play)
        (:Update
          (Rendering|Material|SetScalarParameterValue (Variables|Default|GetMaterialNubesDinamico) "StormClouds" _intensidadtormenta :!class /Script/Engine.MaterialInstanceDynamic))
        (:Finished
          (if (Variables|Default|GetEstaLloviendo)
            (Components|Activation|Activate _niagaracomponent false)
            (else
              (Components|Activation|Deactivate _niagaracomponent))))))
    (elif (Variables|Default|GetEstaLloviendo)
      (Variables|Default|SetEstaLloviendo false)
      (Timeline|TransiciónClima Reverse))))

(event EventBeginPlay
  (bind _returnvalue (Rendering|Material|CreateDynamicMaterialInstance (Utilities|ResolveSoftReference (Variables|/Script/Engine.VolumetricCloudComponent|GetMaterial (Variables|/Script/Engine.VolumetricCloud|GetVolumetricCloudComponent (Variables|Referencias|GetNubes)))) "None" "None" :!class /Script/Engine.KismetMaterialLibrary))
  (bind _output_get (Variables|Default|SetMaterialNubesDinamico _returnvalue))
  (Rendering|Material|SetMaterial (Variables|/Script/Engine.VolumetricCloud|GetVolumetricCloudComponent (Variables|Referencias|GetNubes)) _output_get)
  (Utilities|Time|SetTimerbyEvent (delegate Custom|ComprobarClima) 2.0 true))

(event Collision|EventActorBeginOverlap
  (params (OtherActor :type Actor%20Object%20Reference)))

(event EventTick
  (params (DeltaSeconds :type Float%20%28single-precision%29)))

(fn ConstructionScript)