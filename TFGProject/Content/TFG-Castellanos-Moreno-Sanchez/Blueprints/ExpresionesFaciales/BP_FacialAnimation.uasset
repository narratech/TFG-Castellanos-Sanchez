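; Drives a MetaHuman's facial expression and motion from four personality values (E, N, T, J).
; Weighted, clamped sums of the normalised values yield expression targets and dynamics settings such as blinks, breathing, wiggle and saccades.
; BeginPlay finds the character's head mesh and overrides its post-process AnimBP.
; Each tick interpolates toward the targets and sends both settings structs to that AnimBP through BPI_FacialAnimation.
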(event EventBeginPlay
  ;[0.15 0.15 0.15 0.5] Setup
  (bind _dynamicssettings (CallFunction|CalculateDynamicSettigns))
  (bind _output_get (Variables|Default|SetAuxDynSettings _dynamicssettings))
  (bind _personality (CallFunction|CalculateFaceTargets))
  (Variables|Default|SetAuxPerSettings _personality)
  ;;[0.15 0.15 0.15 0.5] Settings
  (bind (_personalitysettings _settings) (CallFunction|Transfer _personality _output_get))
  (Variables|Default|SetFacialSettings _settings)
  (Variables|Default|SetFacialPersonalitySettings _personalitysettings)
  (bind _metahumanactor (Variables|Default|GetMetahumanActor)
    (:then
      (bind _asdemo_sandbox_character_mover (Utilities|Casting|CastToDemoSandboxCharacter_Mover _metahumanactor))
      (bind _output_get_2 (Variables|Default|SetMetahuman (Variables|/Script/Engine.ChildActorComponent|GetChildActor (Variables|/Game/TFG-Castellanos-Moreno-Sanchez/Blueprints/NPCs/DemoSandboxCharacter_Mover.DemoSandboxCharacter_Mover_C|GetVisualOverride _asdemo_sandbox_character_mover))))
      (CallFunction|FindFace _output_get_2))
    (:else)))

(event EventTick
  (params (DeltaSeconds :type Float%20%28single-precision%29))
  ;[0.8281 0.7723 0 0.9043] Update
  (Variables|Internals|SetIsTicking true)
  (CallFunction|Update DeltaSeconds))

(event EventEndPlay
  (params (EndPlayReason :type EEndPlayReason%20Enum :default "Destroyed"))
  ;[0 0.4041 0.5156] Ended
  (CallFunction|Reset))

(fn ConstructionScript
  (CallFunction|NormPersonality)
  (bind _dynamicssettings (CallFunction|CalculateDynamicSettigns))
  (bind _output_get (Variables|Default|SetAuxDynSettings _dynamicssettings))
  (bind _personality (CallFunction|CalculateFaceTargets))
  (bind _output_get_2 (Variables|Default|SetAuxPerSettings _personality))
  (bind (_personalitysettings _settings) (CallFunction|Transfer _output_get_2 _output_get))
  (Variables|Default|SetFacialPersonalitySettings _personalitysettings)
  (Variables|Default|SetFacialSettings _settings))

(fn CalculateSingleCurvewithRange
  (params (Weight_E :type Float%20%28double-precision%29) (Weight_N :type Float%20%28double-precision%29) (Weight_T :type Float%20%28double-precision%29) (Weight_J :type Float%20%28double-precision%29) (Base_Offset :type Float%20%28double-precision%29) (Min :type Float%20%28double-precision%29) (Max :type Float%20%28double-precision%29))
  (return (Math|Float|Clamp(Float) (+ (+ (+ (+ Base_Offset (* (Variables|Personalidad|GetNorm_E) Weight_E)) (* (Variables|Personalidad|GetNorm_N) Weight_N)) (* (Variables|Personalidad|GetNorm_T) Weight_T)) (* (Variables|Personalidad|GetNorm_J) Weight_J)) Min Max)))

(fn CalculateDynamicSettigns
  (bind _resul_value (CallFunction|CalculateSingleCurvewithRange 1.5 0.0 -0.5 -0.5 1.0 1.0 3.0))
  (bind _resul_value_2 (CallFunction|CalculateSingleCurvewithRange -1e+01 0.0 3e+01 2e+01 2e+01 1.0 1e+02))
  (bind _resul_value_3 (CallFunction|CalculateSingleCurvewithRange 1.0 0.0 -0.3 -0.1 0.5 0.0 5.0))
  (bind _resul_value_4 (CallFunction|CalculateSingleCurvewithRange 0.6 0.4 -0.2 -0.2 0.5 0.1 2.0))
  (return (Utilities|Struct|MakeST_FacialSettings _resul_value _resul_value_2 false 1.0 _resul_value_3 1e+02 _resul_value_4 _resul_value _resul_value_2 false _resul_value_3 1e+02 _resul_value_4 _resul_value _resul_value_2 true _resul_value_3 1e+02 _resul_value_4 _resul_value _resul_value_2 _resul_value _resul_value_2 _resul_value _resul_value_2 true (CallFunction|CalculateSingleCurvewithRange -1.5 -1.0 2.0 0.0 3.5 0.5 8.0) _resul_value _resul_value_2 true (CallFunction|CalculateSingleCurvewithRange 1.0 0.0 -0.5 0.0 1.0 0.1 3.0) (CallFunction|CalculateSingleCurvewithRange 1.0 0.0 0.0 -0.3 1.0 0.1 5.0) (Math|Vector2D|MakeVector2D (CallFunction|CalculateSingleCurvewithRange 15.0 1e+01 0.0 -1e+01 2e+01 5.0 5e+01) (CallFunction|CalculateSingleCurvewithRange 7.5 5.0 0.0 -5.0 1e+01 2.5 25.0)) (Math|Vector2D|MakeVector2D (CallFunction|CalculateSingleCurvewithRange 1.0 2.0 0.0 -0.5 1.0 0.2 5.0) (CallFunction|CalculateSingleCurvewithRange 0.5 1.0 0.0 -0.25 0.5 0.1 2.5)) true "NewEnumerator0" 0.5 0.6 "NewEnumerator0" false)))

(fn CalculateSingleCurve
  (params (Weight_E :type Float%20%28double-precision%29) (Weight_N :type Float%20%28double-precision%29) (Weight_T :type Float%20%28double-precision%29) (Weight_J :type Float%20%28double-precision%29) (Base_Offset :type Float%20%28double-precision%29))
  (return (Math|Float|Clamp(Float) (+ (+ (+ (+ Base_Offset (* (Variables|Personalidad|GetNorm_E) Weight_E)) (* (Variables|Personalidad|GetNorm_N) Weight_N)) (* (Variables|Personalidad|GetNorm_T) Weight_T)) (* (Variables|Personalidad|GetNorm_J) Weight_J)))))

(fn Smoothing
  (params (Current :type Float%20%28double-precision%29) (Target :type Float%20%28double-precision%29) (Time :type Float%20%28double-precision%29))
  (return (Math|Interpolation|FInterpTo Current Target Time (Variables|Personalidad|GetSmoothing_Speed))))

(fn SmoothingAll
  (params (Personality :type ST%20Facial%20Personality%20Settings%20Structure) (Time :type Float%20%28double-precision%29))
  (bind _facialpersonalitysettings (Variables|Default|GetFacialPersonalitySettings))
  (if (> Time 0.0)
    (return (Utilities|Struct|MakeST_FacialPersonalitySettings (Math|Vector2D|MakeVector2D 0.0 (CallFunction|Smoothing (.y (.c_mouth _facialpersonalitysettings)) (.Y (Math|Vector2D|BreakVector2D (.c_mouth Personality))) Time)) (Math|Vector2D|MakeVector2D 0.0 (CallFunction|Smoothing (.y (.c_jaw _facialpersonalitysettings)) (.Y (Math|Vector2D|BreakVector2D (.c_jaw Personality))) Time)) (CallFunction|Smoothing (.blink_eye _facialpersonalitysettings) (.blink_eye Personality) Time) (CallFunction|Smoothing (.brow_lateral _facialpersonalitysettings) (.brow_lateral Personality) Time) (CallFunction|Smoothing (.brow_down _facialpersonalitysettings) (.brow_down Personality) Time) (CallFunction|Smoothing (.brow_raise _facialpersonalitysettings) (.brow_raise Personality) Time) (Math|Vector2D|MakeVector2D 0.0 (CallFunction|Smoothing (.y (.c_eye _facialpersonalitysettings)) (.Y (Math|Vector2D|BreakVector2D (.c_eye Personality))) Time)) (CallFunction|Smoothing (.cheek_raise _facialpersonalitysettings) (.cheek_raise Personality) Time) (Math|Vector2D|MakeVector2D 0.0 (CallFunction|Smoothing (.y (.l_r_nose _facialpersonalitysettings)) (.Y (Math|Vector2D|BreakVector2D (.l_r_nose Personality))) Time)) (CallFunction|Smoothing (.mouth_upper _facialpersonalitysettings) (.mouth_upper Personality) Time) (CallFunction|Smoothing (.mouth_corner_pull _facialpersonalitysettings) (.mouth_corner_pull Personality) Time) (CallFunction|Smoothing (.mouth_corner_depress _facialpersonalitysettings) (.mouth_corner_depress Personality) Time) (CallFunction|Smoothing (.c_neck _facialpersonalitysettings) (.c_neck Personality) Time) (CallFunction|Smoothing (.mouth_sticky _facialpersonalitysettings) (.mouth_sticky Personality) Time)))))

(fn CalculateFaceTargets
  (return (Utilities|Struct|MakeST_FacialPersonalitySettings (Math|Vector2D|MakeVector2D 0.0 (CallFunction|CalculateSingleCurve -0.3 0.0 -0.2 0.1 0.1)) (Math|Vector2D|MakeVector2D 0.0 (CallFunction|CalculateSingleCurve 0.2 0.1 -0.1 -0.2 0.05)) 0.0 (CallFunction|CalculateSingleCurve -0.2 0.4 0.1 -0.1 0.0) (CallFunction|CalculateSingleCurve -0.2 0.1 0.7 0.3 -0.1) (CallFunction|CalculateSingleCurve 0.3 0.6 -0.2 -0.1 0.0) (Math|Vector2D|MakeVector2D 0.0 (CallFunction|CalculateSingleCurve 0.0 0.3 -0.1 0.0 0.5)) (CallFunction|CalculateSingleCurve 0.7 0.0 -0.1 0.0 0.0) (Math|Vector2D|MakeVector2D 0.0 (CallFunction|CalculateSingleCurve 0.1 0.0 0.2 0.0 0.0)) (CallFunction|CalculateSingleCurve 0.0 0.0 0.3 0.1 0.0) (CallFunction|CalculateSingleCurve 0.8 0.1 -0.2 -0.1 0.0) (CallFunction|CalculateSingleCurve -0.5 0.0 0.2 0.4 0.0) (CallFunction|CalculateSingleCurve -0.4 0.2 0.0 0.0 0.0) (CallFunction|CalculateSingleCurve -0.3 0.0 0.1 0.1 0.0))))

(fn NormPersonality
  (Variables|Personalidad|SetNorm_E (Math|Float|Clamp(Float) (* (+ (Variables|Personalidad|GetPersonality_E) 1.0) 0.5)))
  (Variables|Personalidad|SetNorm_N (Math|Float|Clamp(Float) (* (+ (Variables|Personalidad|GetPersonality_N) 1.0) 0.5)))
  (Variables|Personalidad|SetNorm_J (Math|Float|Clamp(Float) (* (+ (Variables|Personalidad|GetPersonality_J) 1.0) 0.5)))
  (Variables|Personalidad|SetNorm_T (Math|Float|Clamp(Float) (* (+ (Variables|Personalidad|GetNorm_T) 1.0) 0.5))))

(fn Transfer
  (params (Personality :type ST%20Facial%20Personality%20Settings%20Structure) (Dynamics :type ST%20Facial%20Settings%20Structure))
  (return (Utilities|Struct|MakeST_FacialPersonalitySettings (.c_mouth Personality) (.c_jaw Personality) (.blink_eye Personality) (.brow_lateral Personality) (.brow_down Personality) (.brow_raise Personality) (.c_eye Personality) (.cheek_raise Personality) (.l_r_nose Personality) (.mouth_upper Personality) (.mouth_corner_pull Personality) (.mouth_corner_depress Personality) (.c_neck Personality) (.mouth_sticky Personality)) (Utilities|Struct|MakeST_FacialSettings (.brows Dynamics) (.browssmoothing Dynamics) (.browsusedynamics Dynamics) (.settings_global_control Dynamics) (.browswigglestrength Dynamics) (.browswigglesmoothing Dynamics) (.browswigglefrequency Dynamics) (.nose Dynamics) (.nosesmoothing Dynamics) (.noseusedynamics Dynamics) (.nosewigglestrength Dynamics) (.nosewigglesmoothing Dynamics) (.nosewigglefrequency Dynamics) (.cheeks Dynamics) (.cheekssmoothing Dynamics) (.cheeksusedynamics Dynamics) (.cheekswigglestrength Dynamics) (.cheekswigglesmoothing Dynamics) (.cheekswigglefrequency Dynamics) (.mouth Dynamics) (.mouthsmoothing Dynamics) (.jaw Dynamics) (.jawsmoothing Dynamics) (.eyes Dynamics) (.eyessmoothing Dynamics) (.generateblinks Dynamics) (.blinkinterval Dynamics) (.blinks Dynamics) (.blinkssmoothing Dynamics) (.usebreathing Dynamics) (.breathstrength Dynamics) (.breathspeed Dynamics) (.microsaccadicweight Dynamics) (.microsaccadicspeed Dynamics) (.microsaccadicenabled Dynamics) (Variables|Emociones|GetEmotion) 0.5 0.6 "NewEnumerator0" (Variables|Emociones|GetUseEmotion))))

(fn SettingsUpdate
  (params (TargetInst :type Object%20Object%20Reference) (Time :type Float%20%28double-precision%29))
  (bind _personalitysettings (CallFunction|SmoothingAll (Variables|Default|GetAuxPerSettings) Time))
  (bind (_personalitysettings_2 _settings) (CallFunction|Transfer _personalitysettings (Variables|Default|GetAuxDynSettings)))
  (bind _output_get (Variables|Default|SetFacialSettings _settings))
  (bind _output_get_2 (Variables|Default|SetFacialPersonalitySettings _personalitysettings_2))
  (bind _curves (Variables|Default|GetCurves)
    (:then
      (Class|BPIFacialAnimation|Updater(Message) TargetInst _output_get _curves (Variables|Global|GetEnabled) _output_get_2))
    (:else)))

(fn Reset
  ;[0.3906 0 0 0.5] Disable FacialAnim
  (Variables|Internals|SetIsTicking false)
  (Variables|Internals|SetSetupCompleteExt false))

(fn Update
  (params (Time :type Float%20%28double-precision%29))
  ;[0.15 0 0.004088 0.5] Anim Updater
  (Variables|Componentes|GetFaceMesh
    (:then
      (Variables|Internals|GetInternalFaceAnimClass
        (:then
          _)
        (:else
          (bind _facemesh (Variables|Componentes|GetFaceMesh)
            (:then
              (Variables|Internals|SetInternalFaceAnimClass (Class|SkeletalMeshComponent|GetPostProcessInstance _facemesh))
              (bind _internalfaceanimclass (Variables|Internals|GetInternalFaceAnimClass)
                (:then
                  _)
                (:else)))
            (:else))))
      (if (Utilities|DoesObjectImplementInterface (Variables|Internals|GetInternalFaceAnimClass) "/Game/TFG-Castellanos-Moreno-Sanchez/Blueprints/ExpresionesFaciales/BPI_FacialAnimation.BPI_FacialAnimation_C")
        (CallFunction|SettingsUpdate _internalfaceanimclass Time)
        (Variables|Internals|SetIsUpdatingExt false)))
    (:else)))

(fn FindFace
  (params (Metahuman_in :type Actor%20Object%20Reference))
  ;[0 0.5833 0.07276 0.5] Find Face SkeletalMesh
  (Utilities|IsValid Metahuman_in
    (:Is%20Valid
      (if (not (Variables|Internals|GetSetupCompleteExt))
        (for _array_element (Actor|GetComponentsByClass Metahuman_in "/Script/Engine.SkeletalMeshComponent")
          (if (Utilities|Enum|Equal(Enum) (Utilities|GetObjectName _array_element) (Variables|Personaje|GetHeadMeshName))
            (bind _output_get (Variables|Componentes|SetFaceMesh _array_element))
            (bind _asanim_instance (Utilities|Casting|CastToAnimInstanceClass (Variables|Default|GetAnimation_BP)))
            (Class|SkeletalMeshComponent|SetOverridePostProcessAnimBP _output_get _asanim_instance true)))
        (bind _facemesh (Variables|Componentes|GetFaceMesh)
          (:then
            (bind _output_get_2 (Variables|Internals|SetInternalFaceAnimClass (Class|SkeletalMeshComponent|GetPostProcessInstance _facemesh)))
            (if (Utilities|DoesObjectImplementInterface _output_get_2 "/Game/TFG-Castellanos-Moreno-Sanchez/Blueprints/ExpresionesFaciales/BPI_FacialAnimation.BPI_FacialAnimation_C")
              (CallFunction|SettingsUpdate _output_get_2 0.0)
              ;;[0.6 0 0.04823] Run debug commands
              (if (Variables|Default|GetDebug)
                (Development|ExecuteConsoleCommand "a.AnimNode.ControlRig.Debug 1" 0)
                (Development|ExecuteConsoleCommand " ControlRig.EnableDrawInterfaceInGame 1" 0))
              (Variables|Internals|SetSetupCompleteExt true)))
          (:else))))))